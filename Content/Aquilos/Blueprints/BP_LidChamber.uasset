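; BP_LidChamber is a VR lid chamber attached to a socket on a Lid actor, with a hand-slid gate.
; While held, the gate follows the hand each tick, clamped to a spline segment; reaching either end toggles GateStatus and records the step with its time in Global_Arrays.
; An IsOpening flag drives a timeline-animated indicator gate, and motion-controller grab-sphere overlaps show or hide an arrow and set a touch flag.
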(event `/Game/VirtualRealityBP/Blueprints/PickupActorInterface.Pickup`
  (params (AttachTo :type "SceneComponent Object Reference"))
  (set `self.Hand` AttachTo))

(event `/Game/VirtualRealityBP/Blueprints/PickupActorInterface.Drop`
  (`self.Hand`
    (:`then`
      (set `self.Hand` null))
    (:`else`)))

(event `self.ReceiveBeginPlay`
  (`self.K2_AttachToActor` (`self.Lid`) "LidChamberSocket" "SnapToTarget" "SnapToTarget" "KeepWorld" false)
  (`SceneComponent.SetVisibility` (`self.LidGateArrow`) false false)
  (set `PrimitiveComponent.bGenerateOverlapEvents` false (`self.LidGateBox`))
  ;[1 1 1] Fix hand collision bug
  (set `PrimitiveComponent.bGenerateOverlapEvents` false (`self.Box_Collision_Backup`)))

(event `UpdateSliderPosition`
  (bind _spline (`self.Spline`))
  ;[0.5137 1 0.4118] Update knob location according to hand's location
  (bind _hand (`self.Hand`)
    (:`then`
      (`SceneComponent.K2_SetWorldLocation` (`self.Lid Gate`) (`KismetMathLibrary.FindClosestPointOnSegment` (`SceneComponent.K2_GetComponentLocation` _hand) (`SplineComponent.GetLocationAtSplinePoint` _spline 0 "World") (`SplineComponent.GetLocationAtSplinePoint` _spline 1 "World")) false true))
    (:`else`)))

(event `self.ReceiveTick`
  (params (DeltaSeconds :type "Float (single-precision)"))
  (`|ExecutionSequence`
    (:`then_0`
      (`self.UpdateSliderPosition`))
    (:`then_1`
      ;[1 1 1] Update gate status
      (switch `/Game/Aquilos/Blueprints/Enum_Valve_Status` (`self.Gate status`)
        (:`NewEnumerator1`
          (if (== (`SceneComponent.K2_GetComponentLocation` (`self.Lid Gate`)) (`SplineComponent.GetLocationAtSplinePoint` (`self.Spline`) 1 "World") :`ErrorTolerance` 1.0)
            (set `self.Gate status` "NewEnumerator0")
            (`self.StepRecord` 19)))
        (:`NewEnumerator0`
          (if (== (`SceneComponent.K2_GetComponentLocation` (`self.Lid Gate`)) (`SplineComponent.GetLocationAtSplinePoint` (`self.Spline`) 0 "World") :`ErrorTolerance` 1.0)
            (set `self.Gate status` "NewEnumerator1")
            (`self.StepRecord` 20)))))
    (:`then_2`
      ;[1 1 1] Indication Animation
      (if (`self.Is_Opening`)
        (`self.Open_Animation`)
        (else
          (`self.Close_Animation`))))))

(event `Open_Animation`
  ;[1 1 1] Indication Animation
  (bind (_direction _newtrack_0) (`Timeline|Timeline_0` :!label _label)
    (:`Update`
      (`SceneComponent.K2_SetRelativeLocation` (`self.Indication Lid Gate`) (`KismetMathLibrary.MakeVector` 0.0 (`KismetMathLibrary.Lerp` 3.081438 7.596436 _newtrack_0)) false false))))

(event `Close_Animation`
  (goto _label :!via `Reverse`))

(event `self.LidGateBox.OnComponentBeginOverlap`
  (params (OverlappedComponent :type "PrimitiveComponent Object Reference") (OtherActor :type "Actor Object Reference") (OtherComp :type "PrimitiveComponent Object Reference") (OtherBodyIndex :type Integer) (bFromSweep :type Boolean) (SweepResult :type "HitResult Structure (by ref)"))
  ;[1 1 1] Lid Gate Touching Judgement
  (bind _asbp_motion_controller (cast `/Game/VirtualRealityBP/Blueprints/BP_MotionController` OtherActor))
  (if (== (`/Game/VirtualRealityBP/Blueprints/BP_MotionController.GrabSphere` _asbp_motion_controller) OtherComp)
    (set `self.LidGateIsTouching` true)
    (`SceneComponent.SetVisibility` (`self.LidGateArrow`) true false)))

(event `self.LidGateBox.OnComponentEndOverlap`
  (params (OverlappedComponent :type "PrimitiveComponent Object Reference") (OtherActor :type "Actor Object Reference") (OtherComp :type "PrimitiveComponent Object Reference") (OtherBodyIndex :type Integer))
  ;[1 1 1] Lid Gate Touching Judgement
  (bind _asbp_motion_controller (cast `/Game/VirtualRealityBP/Blueprints/BP_MotionController` OtherActor))
  (if (== (`/Game/VirtualRealityBP/Blueprints/BP_MotionController.GrabSphere` _asbp_motion_controller) OtherComp)
    (set `self.LidGateIsTouching` false)
    (`SceneComponent.SetVisibility` (`self.LidGateArrow`) false false)))

(fn `StepRecord`
  (params (Step :type Integer))
  (bind _asglobal_arrays (cast `/Game/CryoVR_GeneralContent/Blueprints/Global_Arrays` (`GameplayStatics.GetGameInstance`)))
  (bind _stepindexrecord (`/Game/CryoVR_GeneralContent/Blueprints/Global_Arrays.StepIndexRecord` _asglobal_arrays))
  (bind _returnvalue (`KismetArrayLibrary.Array_Length` _stepindexrecord))
  (if (> _returnvalue 0)
    (if (!= (`|GetArrayItem` _stepindexrecord (- _returnvalue 1)) Step)
      (`KismetArrayLibrary.Array_Add` _stepindexrecord Step)
      (`KismetArrayLibrary.Array_Add` (`/Game/CryoVR_GeneralContent/Blueprints/Global_Arrays.StepTimeRecord` _asglobal_arrays) (`/Game/CryoVR_GeneralContent/Blueprints/Global_Arrays.GlobalRecordTime` _asglobal_arrays)))))

(fn `UserConstructionScript`)