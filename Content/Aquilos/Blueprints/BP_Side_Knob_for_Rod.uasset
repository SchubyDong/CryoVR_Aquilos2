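; BP_Side_Knob_for_Rod is a hand-operated knob on a rod that rotates between lock and unlock angles and tracks a slider position along a spline.
; Tick updates lock rotation from the hand's look-at pitch, flipped when the rod is not horizontal, then runs lock, slider and valve checks.
; A timeline pulls out and rotates an indication knob when open, reversing otherwise.
; MonitorRodStatus toggles Start/End when the knob reaches either spline point.
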(event `self.ReceiveTick`
  (params (DeltaSeconds :type "Float (single-precision)"))
  (`|ExecutionSequence`
    (:`then_0`
      (`self.UpdateLockRotation`))
    (:`then_1`
      (`self.CheckLock`))
    (:`then_2`
      (`self.UpdateSliderPosition`))
    (:`then_3`
      (`self.CheckSlider`))
    (:`then_4`
      (`self.CheckValve`))
    (:`then_5`
      (if (`self.Is_Open`)
        (`self.PulloutAnimation`)
        (else
          (`self.PushinAnimation`))))))

(event `Monitor Rod Status`
  ;[0.5137 1 0.4118] Check slider status
  (switch `/Game/Aquilos/Blueprints/Enum_Slider_Position` (`self.sliderPosition`)
    (:`NewEnumerator0`
      (if (== (`SceneComponent.K2_GetComponentLocation` (`self.Knob`)) (`SplineComponent.GetLocationAtSplinePoint` (`self.Spline`) 1 "World") :`ErrorTolerance` 0.5)
        (set `self.sliderPosition` "NewEnumerator1")))
    (:`NewEnumerator1`
      (if (== (`SceneComponent.K2_GetComponentLocation` (`self.Knob`)) (`SplineComponent.GetLocationAtSplinePoint` (`self.Spline`) 0 "World") :`ErrorTolerance` 0.5)
        (set `self.sliderPosition` "NewEnumerator0")))))

(event `PulloutAnimation`
  ;[1 1 1] Indication Animation
  (bind (_direction _pullout _rotate) (`Timeline|Timeline_0` :!label _label)
    (:`Update`
      (`SceneComponent.K2_SetRelativeLocation` (`self.Indication_Knob`) (`KismetMathLibrary.MakeVector` 0.0 (`KismetMathLibrary.Lerp` 0.0 4.0 _pullout)) false false)
      (`SceneComponent.K2_SetRelativeRotation` (`self.Indication_Knob`) (`KismetMathLibrary.MakeRotator` 0.0 (`KismetMathLibrary.Lerp` 0.0 -90.0 _rotate)) false false))))

(event `PushinAnimation`
  (goto _label :!via `Reverse`))

(event `self.UpdateLockRotation`
  (bind _knob (`self.Knob`))
  (bind _knob_2 (`self.Knob`))
  (bind (_relativerotation_roll _relativerotation_pitch) (`KismetMathLibrary.BreakRotator` (`SceneComponent.RelativeRotation` _knob)))
  (bind (_relativerotation_roll_2 _relativerotation_pitch_2) (`KismetMathLibrary.BreakRotator` (`SceneComponent.RelativeRotation` _knob_2)))
  (bind (_returnvalue_roll _returnvalue_pitch) (`KismetMathLibrary.BreakRotator` (`SceneComponent.K2_GetComponentRotation` (`StaticMeshActor.StaticMeshComponent` (`self.Rod_Ref`)))))
  (if (`self.ifEnableRotate`)
    (bind _hand (`self.Hand`)
      (:`then`
        ;[1 1 1] Rotation Update
        (if (`KismetMathLibrary.NearlyEqual_FloatFloat` _returnvalue_pitch 0.0 5.0)
          (bind (_returnvalue_roll_2 _returnvalue_pitch_2) (`KismetMathLibrary.BreakRotator` (`KismetMathLibrary.FindLookAtRotation` (`SceneComponent.K2_GetComponentLocation` (`self.Knob`)) (`SceneComponent.K2_GetComponentLocation` _hand))))
          (`SceneComponent.K2_SetRelativeRotation` _knob (`KismetMathLibrary.MakeRotator` 0.0 (`KismetMathLibrary.FClamp` (+ _relativerotation_pitch _returnvalue_pitch_2) (`self.unlockAngle`) (`self.lockAngle`))) false true)
          (else
            (bind (_returnvalue_roll_3 _returnvalue_pitch_3) (`KismetMathLibrary.BreakRotator` (`KismetMathLibrary.FindLookAtRotation` (`SceneComponent.K2_GetComponentLocation` _hand) (`SceneComponent.K2_GetComponentLocation` (`self.Knob`)))))
            (`SceneComponent.K2_SetRelativeRotation` _knob_2 (`KismetMathLibrary.MakeRotator` 0.0 (`KismetMathLibrary.FClamp` (+ _relativerotation_pitch_2 _returnvalue_pitch_3) (`self.unlockAngle`) (`self.lockAngle`))) false true))))
      (:`else`))))

(fn `UserConstructionScript`
  (`parent.UserConstructionScript`))