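; Hand-grabbed fixing knob that locks and unlocks by rotation, recording procedure steps.
; While held, Tick turns the knob toward the hand, clamped between unlock and lock angles; nearing either limit flips LockStatus.
; When the referenced left and right knobs match after a flip, an Aquilos-dependent step is appended to the GameInstance's record, skipping consecutive repeats.
; A separate IsLocking flag drives the indication knob's timeline animation.
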(event `/Game/VirtualRealityBP/Blueprints/PickupActorInterface.Pickup`
  (params (AttachTo :type "SceneComponent Object Reference"))
  (set `self.Hand` AttachTo))

(event `/Game/VirtualRealityBP/Blueprints/PickupActorInterface.Drop`
  (`/Engine/EditorBlueprintResources/StandardMacros.IsValid` (`self.Hand`)
    (:`Is Valid`
      (set `self.Hand` null))))

(event `self.ReceiveTick`
  (params (DeltaSeconds :type "Float (single-precision)"))
  (bind _knob (`self.Knob`))
  (bind _leftfixingknob (`self.LeftFixingKnob`))
  (bind _leftfixingknob_2 (`self.LeftFixingKnob`))
  (bind _relativerotation_roll (`KismetMathLibrary.BreakRotator` (`SceneComponent.RelativeRotation` (`self.Knob`))))
  (bind _relativerotation_roll_2 (`KismetMathLibrary.BreakRotator` (`SceneComponent.RelativeRotation` (`self.Knob`))))
  (bind _relativerotation_roll_3 (`KismetMathLibrary.BreakRotator` (`SceneComponent.RelativeRotation` _knob)))
  (`|ExecutionSequence`
    (:`then_0`
      ;[1 1 1] Update actor rotation (roll) according to hand position
      (bind _hand (`self.Hand`)
        (:`then`
          (if (`self.Is_Rotation_Allowed`)
            (bind (_returnvalue_roll _returnvalue_pitch) (`KismetMathLibrary.BreakRotator` (`KismetMathLibrary.FindLookAtRotation` (`SceneComponent.K2_GetComponentLocation` (`self.Knob`)) (`SceneComponent.K2_GetComponentLocation` _hand))))
            (`SceneComponent.K2_SetRelativeRotation` _knob (`KismetMathLibrary.MakeRotator` (`KismetMathLibrary.FClamp` (select `bool` (`self.ifLockDirectionDown`) :`false` (+ _relativerotation_roll_3 _returnvalue_pitch) :`true` (- _relativerotation_roll_3 _returnvalue_pitch)) (`self.unlockAngle`) (`self.lockAngle`))) false true)))
        (:`else`)))
    (:`then_1`
      ;[1 1 1] Check knob status
      (switch `/Game/Aquilos/Blueprints/Enum_Lock_Status` (`self.lockStatus`)
        (:`NewEnumerator0`
          (if (`KismetMathLibrary.NearlyEqual_FloatFloat` _relativerotation_roll_2 (`self.unlockAngle`) 3.0)
            (set `self.lockStatus` "NewEnumerator1")
            (`/Engine/EditorBlueprintResources/StandardMacros.IsValid` _leftfixingknob_2
              (:`Is Valid`
                (if (and (`|EnumEquality` (`/Game/Aquilos/Blueprints/BP_Fixing_Knob.lockStatus` _leftfixingknob_2) "NewEnumerator1") (`|EnumEquality` (`/Game/Aquilos/Blueprints/BP_Fixing_Knob.lockStatus` (`self.RightFixingKnob`)) "NewEnumerator1"))
                  (if (`self.isAquilosKnob`)
                    (`self.StepRecord` 12)
                    (else
                      (`self.StepRecord` 38))))))))
        (:`NewEnumerator1`
          (if (`KismetMathLibrary.NearlyEqual_FloatFloat` _relativerotation_roll (`self.lockAngle`) 3.0)
            (set `self.lockStatus` "NewEnumerator0")
            (`/Engine/EditorBlueprintResources/StandardMacros.IsValid` _leftfixingknob
              (:`Is Valid`
                (if (and (`|EnumEquality` (`/Game/Aquilos/Blueprints/BP_Fixing_Knob.lockStatus` _leftfixingknob) "NewEnumerator0") (`|EnumEquality` (`/Game/Aquilos/Blueprints/BP_Fixing_Knob.lockStatus` (`self.RightFixingKnob`)) "NewEnumerator0"))
                  (if (`self.isAquilosKnob`)
                    (`self.StepRecord` 41)
                    (else
                      (`self.StepRecord` 15))))))))))
    (:`then_2`
      ;[1 1 1] Lock/Unlock Animation
      (if (`self.Is_Locking`)
        (`self.LockRodAnimation`)
        (else
          (`self.UnlockRodAnimation`))))))

(event `UnlockRodAnimation`
  ;[1 1 1] Lock/Unlock Animation
  (bind (_direction _alpha) (`Timeline|Timeline_0` :!label _label)
    (:`Update`
      (`SceneComponent.K2_SetRelativeRotation` (`self.Indication_Knob`) (`KismetMathLibrary.MakeRotator` (`KismetMathLibrary.Lerp` 0.0 -90.0 _alpha)) false false))))

(event `LockRodAnimation`
  (goto _label :!via `Reverse`))

(fn `StepRecord`
  (params (Step :type Integer))
  (bind _asglobal_arrays (cast `/Game/CryoVR_GeneralContent/Blueprints/Global_Arrays` (`GameplayStatics.GetGameInstance`)))
  (bind _stepindexrecord (`/Game/CryoVR_GeneralContent/Blueprints/Global_Arrays.StepIndexRecord` _asglobal_arrays))
  (bind _returnvalue (`KismetArrayLibrary.Array_Length` _stepindexrecord))
  (if (> _returnvalue 0)
    (if (!= (`|GetArrayItem` _stepindexrecord (- _returnvalue 1)) Step)
      (`KismetArrayLibrary.Array_Add` _stepindexrecord Step))))

(fn `UserConstructionScript`)