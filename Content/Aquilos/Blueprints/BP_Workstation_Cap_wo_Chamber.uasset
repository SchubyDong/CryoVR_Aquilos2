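; VR workstation cap Blueprint that starts snapped to the workstation's CapSocket and tracks whether it is capped.
; Tick records step 21 once a grasping motion controller has pulled it clear of the workstation, then pauses ticking for one second.
; Overlapping a Cell_BP snaps it back and marks it capped.
; CapBox overlaps with the hand's GrabSphere toggle the knob arrow and touch flag, though CapBox overlap events start disabled.
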(event `self.ReceiveBeginPlay`
  (`parent.ReceiveBeginPlay`)
  (`self.K2_AttachToComponent` (`StaticMeshActor.StaticMeshComponent` (`self.Workstation`)) "CapSocket" "SnapToTarget" "SnapToTarget" "KeepWorld")
  (set `self.Is_Capped` true)
  (`SceneComponent.SetVisibility` (`self.Knob_Arrow`) false false)
  (set `PrimitiveComponent.bGenerateOverlapEvents` false (`self.Cap_Box`)))

(event `self.ReceiveTick`
  (params (DeltaSeconds :type "Float (single-precision)"))
  (`parent.ReceiveTick` DeltaSeconds)
  (bind _current_hand (`self.Current_Hand`)
    (:`then`
      (if (`/Game/VirtualRealityBP/Blueprints/BP_MotionController.isGrasp` _current_hand)
        (if (and (== (`KismetArrayLibrary.Array_Length` (`PrimitiveComponent.GetOverlappingActors` (`self.StaticMeshComponent`) "/Game/Aquilos/Blueprints/BP_Workstation.BP_Workstation_C")) 0) (`self.Is_Capped`))
          (set `self.Is_Capped` false)
          (`self.StepRecord` 21)
          (`self.SetActorTickEnabled` false)
          (`KismetSystemLibrary.Delay` 1.0)
          (`self.SetActorTickEnabled` true))))
    (:`else`)))

(event `self.StaticMeshComponent.OnComponentEndOverlap`
  (params (OverlappedComponent :type "PrimitiveComponent Object Reference") (OtherActor :type "Actor Object Reference") (OtherComp :type "PrimitiveComponent Object Reference") (OtherBodyIndex :type Integer))
  ;[1 1 1] If hand touched
  (cast `/Game/VirtualRealityBP/Blueprints/BP_MotionController` OtherActor)
  (set `self.Current_Hand` null))

(event `self.StaticMeshComponent.OnComponentBeginOverlap`
  (params (OverlappedComponent :type "PrimitiveComponent Object Reference") (OtherActor :type "Actor Object Reference") (OtherComp :type "PrimitiveComponent Object Reference") (OtherBodyIndex :type Integer) (bFromSweep :type Boolean) (SweepResult :type "HitResult Structure (by ref)"))
  ;[1 1 1] If hand touched
  (`|ExecutionSequence`
    (:`then_0`
      (bind _asbp_motion_controller (cast `/Game/VirtualRealityBP/Blueprints/BP_MotionController` OtherActor))
      (set `self.Current_Hand` _asbp_motion_controller))
    (:`then_1`
      (cast `/Game/Aquilos/Blueprints/Cell_BP` OtherActor)
      (`self.K2_AttachToComponent` (`StaticMeshActor.StaticMeshComponent` (`self.Workstation`)) "CapSocket" "SnapToTarget" "SnapToTarget" "KeepWorld")
      (set `self.Is_Capped` true))))

(event `self.Cap_Box.OnComponentBeginOverlap`
  (params (OverlappedComponent :type "PrimitiveComponent Object Reference") (OtherActor :type "Actor Object Reference") (OtherComp :type "PrimitiveComponent Object Reference") (OtherBodyIndex :type Integer) (bFromSweep :type Boolean) (SweepResult :type "HitResult Structure (by ref)"))
  ;[1 1 1] CapTouchingJudgement
  (bind _asbp_motion_controller (cast `/Game/VirtualRealityBP/Blueprints/BP_MotionController` OtherActor))
  (if (== (`/Game/VirtualRealityBP/Blueprints/BP_MotionController.GrabSphere` _asbp_motion_controller) OtherComp)
    (set `self.CapIsTouching` true)
    (`SceneComponent.SetVisibility` (`self.Knob_Arrow`) true false)))

(event `self.Cap_Box.OnComponentEndOverlap`
  (params (OverlappedComponent :type "PrimitiveComponent Object Reference") (OtherActor :type "Actor Object Reference") (OtherComp :type "PrimitiveComponent Object Reference") (OtherBodyIndex :type Integer))
  ;[1 1 1] CapTouchingJudgement
  (bind _asbp_motion_controller (cast `/Game/VirtualRealityBP/Blueprints/BP_MotionController` OtherActor))
  (if (== (`/Game/VirtualRealityBP/Blueprints/BP_MotionController.GrabSphere` _asbp_motion_controller) OtherComp)
    (set `self.CapIsTouching` false)
    (`SceneComponent.SetVisibility` (`self.Knob_Arrow`) false false)))

(fn `UserConstructionScript`
  (`parent.UserConstructionScript`))