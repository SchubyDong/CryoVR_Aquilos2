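; BP_Workstation_Cap is a cap for a workstation in what appears to be a VR setup, tracking whether it is still in place.
; On BeginPlay it snaps onto the referenced Workstation mesh's CapSocket, keeping world scale, and sets IsCapped.
; A BP_MotionController overlapping the cap's mesh clears IsCapped; this graph only changes the flag and does not detach the cap.
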(event `self.ReceiveBeginPlay`
  (`parent.ReceiveBeginPlay`)
  (`self.K2_AttachToComponent` (`StaticMeshActor.StaticMeshComponent` (`self.Workstation`)) "CapSocket" "SnapToTarget" "SnapToTarget" "KeepWorld")
  (set `self.Is_Capped` true))

(event `self.ReceiveTick`
  (params (DeltaSeconds :type "Float (single-precision)"))
  (`parent.ReceiveTick` DeltaSeconds))

(event `self.StaticMeshComponent.OnComponentBeginOverlap`
  (params (OverlappedComponent :type "PrimitiveComponent Object Reference") (OtherActor :type "Actor Object Reference") (OtherComp :type "PrimitiveComponent Object Reference") (OtherBodyIndex :type Integer) (bFromSweep :type Boolean) (SweepResult :type "HitResult Structure (by ref)"))
  (cast `/Game/VirtualRealityBP/Blueprints/BP_MotionController` OtherActor)
  (set `self.Is_Capped` false))

(fn `UserConstructionScript`
  (`parent.UserConstructionScript`))