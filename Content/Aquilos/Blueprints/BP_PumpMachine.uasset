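; BP_PumpMachine is a VR pump machine with mutually exclusive Pumping and Venting buttons, pressed by a motion controller's index finger.
; A proximity box switches empty hands to an index-finger-only gesture near the buttons.
; Each press starts a frame-counted Tick timer that shows status text, then logs the completed step and time to Global_Arrays, skipping consecutive repeats.
; BeginPlay passes a self reference to both UI widgets.
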(event `self.ReceiveBeginPlay`
  (`SceneComponent.SetVisibility` (`self.PumpingText`) false true)
  (bind _aspumping_ui (cast `/Game/Aquilos/UI/Pumping_UI` (`WidgetComponent.GetUserWidgetObject` (`self.PumpingUI`))))
  (set `/Game/Aquilos/UI/Pumping_UI.Pump_Machine` self _aspumping_ui)
  (`SceneComponent.SetVisibility` (`self.VentingText`) false true)
  (bind _asventing_ui (cast `/Game/Aquilos/UI/Venting_UI` (`WidgetComponent.GetUserWidgetObject` (`self.VentingUI`))))
  (set `/Game/Aquilos/UI/Venting_UI.Pump_Machine` self _asventing_ui))

(event `self.Box_Button_Hand_Gesture.OnComponentBeginOverlap`
  (params (OverlappedComponent :type "PrimitiveComponent Object Reference") (OtherActor :type "Actor Object Reference") (OtherComp :type "PrimitiveComponent Object Reference") (OtherBodyIndex :type Integer) (bFromSweep :type Boolean) (SweepResult :type "HitResult Structure (by ref)"))
  ;[1 1 1] Change empty hand gesture if close to buttons
  (bind _asbp_motion_controller (cast `/Game/VirtualRealityBP/Blueprints/BP_MotionController` OtherActor))
  (if (and (== (`/Game/VirtualRealityBP/Blueprints/BP_MotionController.IndexFingerColli` _asbp_motion_controller) OtherComp) (not (`/Game/VirtualRealityBP/Blueprints/BP_MotionController.isGrasp` _asbp_motion_controller)))
    (set `/Game/VirtualRealityBP/Blueprints/BP_MotionController.ifOnlyIndexFinger` true _asbp_motion_controller)))

(event `self.Box_Button_Hand_Gesture_exit.OnComponentEndOverlap`
  (params (OverlappedComponent :type "PrimitiveComponent Object Reference") (OtherActor :type "Actor Object Reference") (OtherComp :type "PrimitiveComponent Object Reference") (OtherBodyIndex :type Integer))
  ;[1 1 1] Change empty hand gesture if close to buttons
  (bind _asbp_motion_controller (cast `/Game/VirtualRealityBP/Blueprints/BP_MotionController` OtherActor))
  (set `/Game/VirtualRealityBP/Blueprints/BP_MotionController.ifOnlyIndexFinger` false _asbp_motion_controller))

(event `self.Pumping_BoxCollision.OnComponentBeginOverlap`
  (params (OverlappedComponent :type "PrimitiveComponent Object Reference") (OtherActor :type "Actor Object Reference") (OtherComp :type "PrimitiveComponent Object Reference") (OtherBodyIndex :type Integer) (bFromSweep :type Boolean) (SweepResult :type "HitResult Structure (by ref)"))
  ;[1 1 1] Vent & Pump (Need future actions to prevent mistouch)
  (bind _asbp_motion_controller (cast `/Game/VirtualRealityBP/Blueprints/BP_MotionController` OtherActor))
  (if (and (== (`/Game/VirtualRealityBP/Blueprints/BP_MotionController.IndexFingerColli` _asbp_motion_controller) OtherComp) (not (`self.IsVenting`)))
    (set `self.IsPumping` true)))

(event `self.Venting_BoxCollision.OnComponentBeginOverlap`
  (params (OverlappedComponent :type "PrimitiveComponent Object Reference") (OtherActor :type "Actor Object Reference") (OtherComp :type "PrimitiveComponent Object Reference") (OtherBodyIndex :type Integer) (bFromSweep :type Boolean) (SweepResult :type "HitResult Structure (by ref)"))
  ;[1 1 1] Vent & Pump (Need future actions to prevent mistouch)
  (bind _asbp_motion_controller (cast `/Game/VirtualRealityBP/Blueprints/BP_MotionController` OtherActor))
  (if (and (== (`/Game/VirtualRealityBP/Blueprints/BP_MotionController.IndexFingerColli` _asbp_motion_controller) OtherComp) (not (`self.IsPumping`)))
    (set `self.IsVenting` true)))

(event `self.ReceiveTick`
  (params (DeltaSeconds :type "Float (single-precision)"))
  (`|ExecutionSequence`
    (:`then_0`
      (if (and (`self.IsPumping`) (not (`self.IsVenting`)))
        (`SceneComponent.SetVisibility` (`self.PumpingText`) true true)
        (`/Engine/EditorBlueprintResources/StandardMacros.IncrementInt` (`self.Pumping_Time`)
          (:`  `
            (if (>= (`self.Pumping_Time`) 300)
              (set `self.IsPumping` false)
              (set `self.Pumping_Time` 0)
              (`self.StepRecord` 17)
              (`SceneComponent.SetVisibility` (`self.PumpingText`) false true))))))
    (:`then_1`
      (if (and (`self.IsVenting`) (not (`self.IsPumping`)))
        (`SceneComponent.SetVisibility` (`self.VentingText`) true true)
        (`/Engine/EditorBlueprintResources/StandardMacros.IncrementInt` (`self.Venting_Time`)
          (:`  `
            (if (>= (`self.Venting_Time`) 300)
              (set `self.IsVenting` false)
              (set `self.Venting_Time` 0)
              (`self.StepRecord` 18)
              (`SceneComponent.SetVisibility` (`self.VentingText`) false true))))))))

(fn `StepRecord`
  (params (Step :type Integer))
  (bind _asglobal_arrays (cast `/Game/CryoVR_GeneralContent/Blueprints/Global_Arrays` (`GameplayStatics.GetGameInstance`)))
  (bind _stepindexrecord (`/Game/CryoVR_GeneralContent/Blueprints/Global_Arrays.StepIndexRecord` _asglobal_arrays))
  (bind _returnvalue (`KismetArrayLibrary.Array_Length` _stepindexrecord))
  (if (> _returnvalue 0)
    (if (!= (`|GetArrayItem` _stepindexrecord (- _returnvalue 1)) Step)
      (`KismetArrayLibrary.Array_Add` _stepindexrecord Step)
      (`KismetArrayLibrary.Array_Add` (`/Game/CryoVR_GeneralContent/Blueprints/Global_Arrays.StepTimeRecord` _asglobal_arrays) (`/Game/CryoVR_GeneralContent/Blueprints/Global_Arrays.GlobalRecordTime` _asglobal_arrays)))))

(fn `UserConstructionScript`)