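; Workstation actor for a step-based lab procedure where tools cool a pod, flip the shuttle and handle the grid box.
; Collision overlaps snap tools and cap to sockets and advance status enums, faking part hand-offs by toggling mesh visibility behind DoOnce-and-Delay debounces.
; Tick checks socket occupancy, counts cooling per frame and animates the screwdriver indicator.
; StepRecord appends completed steps to the GameInstance's non-empty history, skipping consecutive duplicates.
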(event `self.ReceiveBeginPlay`
  (`SceneComponent.SetVisibility` (`self.CoolingText`) false true)
  (bind _ascooldown_ui (cast `/Game/Aquilos/UI/Cooldown_UI` (`WidgetComponent.GetUserWidgetObject` (`self.CoolingUI`))))
  (set `/Game/Aquilos/UI/Cooldown_UI.WorkstationRef` self _ascooldown_ui)
  (for _array_element (`SceneComponent.GetChildrenComponents` (`self.StaticMeshComponent`) false)
    (bind _asprimitive_component (cast `PrimitiveComponent` _array_element))
    (set `PrimitiveComponent.bGenerateOverlapEvents` false _asprimitive_component))
  (set `PrimitiveComponent.bGenerateOverlapEvents` true (`self.Cap_Collision`))
  (set `PrimitiveComponent.bGenerateOverlapEvents` true (`StaticMeshActor.StaticMeshComponent` (`self.Pod_Cap`))))

(event `self.Cap_Collision.OnComponentBeginOverlap`
  (params (OverlappedComponent :type "PrimitiveComponent Object Reference") (OtherActor :type "Actor Object Reference") (OtherComp :type "PrimitiveComponent Object Reference") (OtherBodyIndex :type Integer) (bFromSweep :type Boolean) (SweepResult :type "HitResult Structure (by ref)"))
  (bind _pod_cap (`self.Pod_Cap`))
  ;[1 1 1] Step 11 Open Cap/Lid
  (bind _asbp_workstation_cap (cast `/Game/Aquilos/Blueprints/BP_Workstation_Cap` OtherActor))
  (switch `/Game/Aquilos/Blueprints/Enum_ToolSockets_Status` (`self.SocketsStatus`)
    (:`NewEnumerator2`
      (`self.K2_AttachToComponent` _asbp_workstation_cap (`self.StaticMeshComponent`) "CapSocket" "SnapToTarget" "SnapToTarget" "KeepWorld" true)
      (for _array_element (`SceneComponent.GetChildrenComponents` (`self.StaticMeshComponent`) false)
        (bind _asprimitive_component (cast `PrimitiveComponent` _array_element))
        (set `PrimitiveComponent.bGenerateOverlapEvents` false _asprimitive_component))
      (set `PrimitiveComponent.bGenerateOverlapEvents` true (`self.Cap_Collision`))
      (set `PrimitiveComponent.bGenerateOverlapEvents` true (`StaticMeshActor.StaticMeshComponent` _pod_cap))
      (set `/Game/Aquilos/Blueprints/BP_Workstation_Cap.Is_Capped` true _pod_cap)
      (set `/Game/Aquilos/Blueprints/BP_Workstation_Cap.Current_Hand` null _pod_cap)
      (`self.StepRecord` 36))))

(event `self.Cap_Collision.OnComponentEndOverlap`
  (params (OverlappedComponent :type "PrimitiveComponent Object Reference") (OtherActor :type "Actor Object Reference") (OtherComp :type "PrimitiveComponent Object Reference") (OtherBodyIndex :type Integer))
  ;[1 1 1] Step 11 Open Cap/Lid
  (cast `/Game/Aquilos/Blueprints/BP_Workstation_Cap` OtherActor)
  (for _array_element (`SceneComponent.GetChildrenComponents` (`self.StaticMeshComponent`) false)
    (bind _asprimitive_component (cast `PrimitiveComponent` _array_element))
    (set `PrimitiveComponent.bGenerateOverlapEvents` true _asprimitive_component)))

(event `self.ScrewDriver_Collision.OnComponentBeginOverlap`
  (params (OverlappedComponent :type "PrimitiveComponent Object Reference") (OtherActor :type "Actor Object Reference") (OtherComp :type "PrimitiveComponent Object Reference") (OtherBodyIndex :type Integer) (bFromSweep :type Boolean) (SweepResult :type "HitResult Structure (by ref)"))
  ;[1 1 1] Step 12 Cool down 3 tools
  (bind _asbp_screw_driver (cast `/Game/Aquilos/Blueprints/BP_ScrewDriver` OtherActor))
  (`self.K2_AttachToComponent` _asbp_screw_driver (`self.StaticMeshComponent`) "ScrewDriverSocket" "SnapToTarget" "SnapToTarget" "KeepWorld" true))

(event `self.ClipPen_Collision.OnComponentBeginOverlap`
  (params (OverlappedComponent :type "PrimitiveComponent Object Reference") (OtherActor :type "Actor Object Reference") (OtherComp :type "PrimitiveComponent Object Reference") (OtherBodyIndex :type Integer) (bFromSweep :type Boolean) (SweepResult :type "HitResult Structure (by ref)"))
  ;[1 1 1] Step 12 Cool down 3 tools
  (bind _asbp_clippen (cast `/Game/Aquilos/Blueprints/BP_Clippen` OtherActor))
  (`self.K2_AttachToComponent` _asbp_clippen (`self.StaticMeshComponent`) "CapPenSocket" "SnapToTarget" "SnapToTarget" "KeepWorld" true))

(event `self.Tweezers_Collision.OnComponentBeginOverlap`
  (params (OverlappedComponent :type "PrimitiveComponent Object Reference") (OtherActor :type "Actor Object Reference") (OtherComp :type "PrimitiveComponent Object Reference") (OtherBodyIndex :type Integer) (bFromSweep :type Boolean) (SweepResult :type "HitResult Structure (by ref)"))
  ;[1 1 1] Step 12 Cool down 3 tools
  (bind _asbp_tweezers (cast `/Game/Aquilos/Blueprints/BP_Tweezers` OtherActor))
  (`self.K2_AttachToComponent` _asbp_tweezers (`self.StaticMeshComponent`) "TweezersSocket" "SnapToTarget" "SnapToTarget" "KeepWorld" true))

(event `self.Shuttle_Collision.OnComponentBeginOverlap`
  (params (OverlappedComponent :type "PrimitiveComponent Object Reference") (OtherActor :type "Actor Object Reference") (OtherComp :type "PrimitiveComponent Object Reference") (OtherBodyIndex :type Integer) (bFromSweep :type Boolean) (SweepResult :type "HitResult Structure (by ref)"))
  (bind _screwdriver_collision (`self.ScrewDriver_Collision`))
  ;[1 1 1] Step 13 Use SD flip the Shuttle
  (cast `/Game/Aquilos/Blueprints/BP_ScrewDriver` OtherActor
    (:`then`
      (`/Engine/EditorBlueprintResources/StandardMacros.DoOnce` false :!label _label
        (:`Completed`
          (switch `/Game/Aquilos/Blueprints/Enum_Shuttle_Status` (`self.ShuttleStatus`)
            (:`NewEnumerator0`
              (`SceneComponent.K2_SetRelativeTransform` (`self.Shuttle`) (`KismetMathLibrary.MakeTransform` (0.0 1.6 3.0) (struct) (0.024 0.024 0.012)) false false)
              (set `PrimitiveComponent.bGenerateOverlapEvents` false _screwdriver_collision)
              (set `self.ShuttleStatus` "NewEnumerator1")
              (`self.StepRecord` 23)
              (`KismetSystemLibrary.Delay` 2.0)
              (set `PrimitiveComponent.bGenerateOverlapEvents` true _screwdriver_collision)
              (`KismetSystemLibrary.Delay` 8.0)
              (goto _label :!via `Reset`))
            (:`NewEnumerator1`
              (switch `/Game/Aquilos/Blueprints/Enum_ShuttleScrew_Status` (`self.ShuttleScrewStatus`)
                (:`NewEnumerator0`
                  (`SceneComponent.K2_SetRelativeTransform` (`self.Shuttle`) (`KismetMathLibrary.MakeTransform` (0.0 -0.4 3.0) (struct :`Roll` -90.0) (0.024 0.024 0.012)) false false)
                  (set `self.ShuttleStatus` "NewEnumerator0")
                  (`self.StepRecord` 31)
                  (`KismetSystemLibrary.Delay` 10.0)
                  (goto _label :!via `Reset`))))))))
    (:`CastFailed`
      ;[1 1 1] Step 19 Attach the grid to the shuttle notch
      (bind _asbp_tweezers (cast `/Game/Aquilos/Blueprints/BP_Tweezers` OtherActor))
      (`/Engine/EditorBlueprintResources/StandardMacros.DoOnce` false :!label _label_2
        (:`Completed`
          (switch `/Game/Aquilos/Blueprints/Enum_Grid_Status` (`self.GridStatus`)
            (:`NewEnumerator1`
              (switch `/Game/Aquilos/Blueprints/Enum_ShuttleScrew_Status` (`self.ShuttleScrewStatus`)
                (:`NewEnumerator1`
                  (`SceneComponent.SetVisibility` (`/Game/Aquilos/Blueprints/BP_Tweezers.Grid` _asbp_tweezers) false false)
                  (`SceneComponent.SetVisibility` (`self.GridOnNotch`) true false)
                  (set `self.GridStatus` "NewEnumerator2")
                  (`self.StepRecord` 29)
                  (`KismetSystemLibrary.Delay` 2.0)
                  (goto _label_2 :!via `Reset`))))))))))

(event `self.ShuttleScrew_Collision.OnComponentBeginOverlap`
  (params (OverlappedComponent :type "PrimitiveComponent Object Reference") (OtherActor :type "Actor Object Reference") (OtherComp :type "PrimitiveComponent Object Reference") (OtherBodyIndex :type Integer) (bFromSweep :type Boolean) (SweepResult :type "HitResult Structure (by ref)"))
  ;[1 1 1] Step 16 & 20 Lossen & Tighten the Shuttle Screw using SD
  (cast `/Game/Aquilos/Blueprints/BP_ScrewDriver` OtherActor)
  (`/Engine/EditorBlueprintResources/StandardMacros.DoOnce` false :!label _label_3
    (:`Completed`
      (switch `/Game/Aquilos/Blueprints/Enum_ShuttleScrew_Status` (`self.ShuttleScrewStatus`)
        (:`NewEnumerator1`
          (set `self.ShuttleScrewStatus` "NewEnumerator0")
          (`self.StepRecord` 30)
          (`SceneComponent.K2_SetRelativeLocation` (`self.ShuttleScrew`) (0.0 -41.666668 38.0) false false))
        (:`NewEnumerator0`
          (set `self.ShuttleScrewStatus` "NewEnumerator1")
          (`self.StepRecord` 26)
          (`SceneComponent.K2_SetRelativeLocation` (`self.ShuttleScrew`) (0.0 -41.666668 62.0) false false)))
      (`KismetSystemLibrary.Delay` 4.0)
      (goto _label_3 :!via `Reset`))))

(event `self.GridBox_Collision.OnComponentBeginOverlap`
  (params (OverlappedComponent :type "PrimitiveComponent Object Reference") (OtherActor :type "Actor Object Reference") (OtherComp :type "PrimitiveComponent Object Reference") (OtherBodyIndex :type Integer) (bFromSweep :type Boolean) (SweepResult :type "HitResult Structure (by ref)"))
  ;[1 1 1] Step 15 Put gridbox from freezedewar tweezer into pod
  (bind _asbp_freeze_dewar_tweezer (cast `/Game/Aquilos/Blueprints/BP_Freeze_Dewar_Tweezer` OtherActor)
    (:`then`
      (`/Engine/EditorBlueprintResources/StandardMacros.DoOnce` false :!label _label_4
        (:`Completed`
          (switch `/Game/Aquilos/Blueprints/Enum_GridBox_Status` (`self.GridBoxStatus`)
            (:`NewEnumerator1`
              (`SceneComponent.SetVisibility` (`/Game/Aquilos/Blueprints/BP_Freeze_Dewar_Tweezer.GridBox` _asbp_freeze_dewar_tweezer) false false)
              (`SceneComponent.SetVisibility` (`/Game/Aquilos/Blueprints/BP_Freeze_Dewar_Tweezer.GridBoxCap` _asbp_freeze_dewar_tweezer) false false)
              (`SceneComponent.SetVisibility` (`self.GridBox`) true false)
              (`SceneComponent.SetVisibility` (`self.GridBoxCap`) true false)
              (set `self.GridBoxStatus` "NewEnumerator2")
              (`self.StepRecord` 25)
              (`KismetSystemLibrary.Delay` 1.0)
              (goto _label_4 :!via `Reset`))
            (:`NewEnumerator2`
              ;[1 1 1] Step 23 Use freeze dewar tweezer pickup the gridbox
              (`SceneComponent.SetVisibility` (`/Game/Aquilos/Blueprints/BP_Freeze_Dewar_Tweezer.GridBox` _asbp_freeze_dewar_tweezer) true false)
              (`SceneComponent.SetVisibility` (`/Game/Aquilos/Blueprints/BP_Freeze_Dewar_Tweezer.GridBoxCap` _asbp_freeze_dewar_tweezer) true false)
              (`SceneComponent.SetVisibility` (`self.GridBox`) false false)
              (`SceneComponent.SetVisibility` (`self.GridBoxCap`) false false)
              (set `self.GridBoxStatus` "NewEnumerator1")
              (`self.StepRecord` 33)
              (`KismetSystemLibrary.Delay` 1.0)
              (goto _label_4 :!via `Reset`))))))
    (:`CastFailed`
      ;[1 1 1] Step 17 Uncap the gridbox by clippen
      (bind _asbp_clippen (cast `/Game/Aquilos/Blueprints/BP_Clippen` OtherActor)
        (:`then`
          (`/Engine/EditorBlueprintResources/StandardMacros.DoOnce` false :!label _label_5
            (:`Completed`
              (switch `/Game/Aquilos/Blueprints/Enum_GridBox_Status` (`self.GridBoxStatus`)
                (:`NewEnumerator2`
                  (`SceneComponent.SetVisibility` (`self.GridBoxCap`) false false)
                  (`SceneComponent.SetVisibility` (`/Game/Aquilos/Blueprints/BP_Clippen.GridBoxCap` _asbp_clippen) true false)
                  (`SceneComponent.SetVisibility` (`self.Grid`) true false)
                  (set `self.GridBoxStatus` "NewEnumerator3")
                  (`self.StepRecord` 27)
                  (`KismetSystemLibrary.Delay` 1.0)
                  (goto _label_5 :!via `Reset`))
                (:`NewEnumerator3`
                  ;[1 1 1] Step 22 Cap the gridbox
                  (`SceneComponent.SetVisibility` (`self.GridBoxCap`) true false)
                  (`SceneComponent.SetVisibility` (`/Game/Aquilos/Blueprints/BP_Clippen.GridBoxCap` _asbp_clippen) false false)
                  (set `self.GridBoxStatus` "NewEnumerator2")
                  (`self.StepRecord` 32)
                  (`KismetSystemLibrary.Delay` 1.0)
                  (goto _label_5 :!via `Reset`))))))
        (:`CastFailed`
          ;[1 1 1] Step 18 Grab the grid with tweezer
          (bind _asbp_tweezers (cast `/Game/Aquilos/Blueprints/BP_Tweezers` OtherActor))
          (`/Engine/EditorBlueprintResources/StandardMacros.DoOnce` false :!label _label_6
            (:`Completed`
              (switch `/Game/Aquilos/Blueprints/Enum_Grid_Status` (`self.GridStatus`)
                (:`NewEnumerator0`
                  (`SceneComponent.SetVisibility` (`self.Grid`) false false)
                  (`SceneComponent.SetVisibility` (`/Game/Aquilos/Blueprints/BP_Tweezers.Grid` _asbp_tweezers) true false)
                  (set `self.GridStatus` "NewEnumerator1")
                  (`self.StepRecord` 28)
                  (`KismetSystemLibrary.Delay` 1.0)
                  (goto _label_6 :!via `Reset`))))))))))

(event `self.ReceiveTick`
  (params (DeltaSeconds :type "Float (single-precision)"))
  (`self.SetSocketsStatus`)
  ;[1 1 1] Screw Driver Animation
  (if (`SceneComponent.IsVisible` (`self.IndicationScrewDriver`))
    (bind (_direction _newtrack_0) (`Timeline|Shuttle Screw Indication Animation`)
      (:`Update`
        (`SceneComponent.K2_SetRelativeLocation` (`self.IndicationScrewDriver`) (`KismetMathLibrary.MakeVector` 0.0 0.0 (`KismetMathLibrary.Lerp` 3411.0 3691.0 _newtrack_0)) false false)))))

(fn `SetSocketsStatus`
  (if (and (`PrimitiveComponent.IsOverlappingComponent` (`self.ScrewDriver_Collision`) (`StaticMeshActor.StaticMeshComponent` (`self.Screw_Ref`))) (`PrimitiveComponent.IsOverlappingComponent` (`self.Tweezers_Collision`) (`StaticMeshActor.StaticMeshComponent` (`self.Tweezer_Ref`))) (`PrimitiveComponent.IsOverlappingComponent` (`self.ClipPen_Collision`) (`StaticMeshActor.StaticMeshComponent` (`self.Clippen_Ref`))))
    (set `self.SocketsStatus` "NewEnumerator0")
    (set `self.AreToolsAttached` true)
    (set `self.IsCooling` true)
    (if (> (`self.CoolingProgress`) 1000)
      (if (not (`self.isCoolingFinished`))
        (`self.StepRecord` 22)
        (set `self.isCoolingFinished` true))
      (else
        (`/Engine/EditorBlueprintResources/StandardMacros.IncrementInt` (`self.CoolingProgress`))))
    (elif (and (not (`PrimitiveComponent.IsOverlappingComponent` (`self.ScrewDriver_Collision`) (`StaticMeshActor.StaticMeshComponent` (`self.Screw_Ref`)))) (not (`PrimitiveComponent.IsOverlappingComponent` (`self.Tweezers_Collision`) (`StaticMeshActor.StaticMeshComponent` (`self.Tweezer_Ref`)))) (not (`PrimitiveComponent.IsOverlappingComponent` (`self.ClipPen_Collision`) (`StaticMeshActor.StaticMeshComponent` (`self.Clippen_Ref`)))))
      (set `self.SocketsStatus` "NewEnumerator2")
      (if (`self.AreToolsAttached`)
        (set `self.AreToolsAttached` false)
        (`self.StepRecord` 35))
      (else
        (set `self.SocketsStatus` "NewEnumerator1")))))

(fn `StepRecord`
  (params (Step :type Integer))
  (bind _asglobal_arrays (cast `/Game/CryoVR_GeneralContent/Blueprints/Global_Arrays` (`GameplayStatics.GetGameInstance`)))
  (bind _stepindexrecord (`/Game/CryoVR_GeneralContent/Blueprints/Global_Arrays.StepIndexRecord` _asglobal_arrays))
  (bind _returnvalue (`KismetArrayLibrary.Array_Length` _stepindexrecord))
  (if (> _returnvalue 0)
    (if (!= (`|GetArrayItem` _stepindexrecord (- _returnvalue 1)) Step)
      (`KismetArrayLibrary.Array_Add` _stepindexrecord Step))))

(fn `UserConstructionScript`)