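; VR tweezer prop for a freeze dewar that a motion controller can pick up.
; On overlap with a BP_MotionController, it calls UpdateHandAniFunc to configure hand animation and snapping to the Freeze_Tweezer_Socket.
; While the overlap flag is set, Tick copies the controller's grip intent into the picked-up state.
; A custom event clears both the overlap and picked-up flags.
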(event `self.ReceiveBeginPlay`
  (`parent.ReceiveBeginPlay`))

(event `self.ReceiveActorBeginOverlap`
  (params (OtherActor :type "Actor Object Reference"))
  (bind _asbp_motion_controller (cast `/Game/VirtualRealityBP/Blueprints/BP_MotionController` OtherActor))
  (`self.UpdateHandAniFunc` _asbp_motion_controller 0.0 0.5 "Freeze_Tweezer_Socket" "SnapToTarget" (1.0 1.0 1.5) true))

(event `CustomEvent_1`
  (params (OtherActor :type "Actor Object Reference"))
  (set `self.ifBeginOverlap` false)
  (set `self.isSelfPickedup` false))

(event `self.ReceiveTick`
  (params (DeltaSeconds :type "Float (single-precision)"))
  (`parent.ReceiveTick` DeltaSeconds)
  (if (`self.ifBeginOverlap`)
    (set `self.isSelfPickedup` (`/Game/VirtualRealityBP/Blueprints/BP_MotionController.bWantsToGrip` (`self.BP_MotionController`)))))

(fn `UserConstructionScript`
  (`parent.UserConstructionScript`))