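; BP_Tweezers is a VR tweezers tool that a motion controller picks up, with a Grid mesh hidden at start.
; Controller overlap stores the hand and calls UpdateHandAniFunc with a gesture value and snap socket.
; While overlapping, Tick mirrors the controller's grip intent into IsSelfPickedup.
; Disconnected logic, with unresolved casts, would move the grid from its holder to a metal support by toggling visibility; the Sphere overlap currently does nothing.
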(event `self.ReceiveBeginPlay`
  (`parent.ReceiveBeginPlay`)
  (`SceneComponent.SetVisibility` (`self.Grid`) false true))

(event `self.ReceiveActorBeginOverlap`
  (params (OtherActor :type "Actor Object Reference"))
  (bind _asbp_motion_controller (cast `/Game/VirtualRealityBP/Blueprints/BP_MotionController` OtherActor))
  (set `self.BP_MotionController` _asbp_motion_controller)
  (`self.UpdateHandAniFunc` OtherActor 0.0 0.5 "Tweezer_Socket" "SnapToTarget" (1.0 1.0 1.0) true)
  (set `self.ifBeginOverlap` true))

(event `self.ReceiveActorEndOverlap`
  (params (OtherActor :type "Actor Object Reference"))
  (set `self.ifBeginOverlap` false)
  (set `self.isSelfPickedup` false))

(event `self.ReceiveTick`
  (params (DeltaSeconds :type "Float (single-precision)"))
  (`parent.ReceiveTick` DeltaSeconds)
  (if (`self.ifBeginOverlap`)
    (set `self.isSelfPickedup` (`/Game/VirtualRealityBP/Blueprints/BP_MotionController.bWantsToGrip` (`self.BP_MotionController`)))))

(event `self.Sphere.OnComponentBeginOverlap`
  (params (OverlappedComponent :type "PrimitiveComponent Object Reference") (OtherActor :type "Actor Object Reference") (OtherComp :type "PrimitiveComponent Object Reference") (OtherBodyIndex :type Integer) (bFromSweep :type Boolean) (SweepResult :type "HitResult Structure (by ref)")))

(fn `UserConstructionScript`
  (`parent.UserConstructionScript`))