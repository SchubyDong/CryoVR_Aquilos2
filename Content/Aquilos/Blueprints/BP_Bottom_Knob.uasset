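; BP_Bottom_Knob is a hand-turned knob that switches between locked and unlocked states.
; Pickup stores the grabbing hand and Drop clears it.
; While held, Tick adjusts the knob's roll from the look-at pitch between knob and hand, reversing the look-at direction by the referenced rod's pitch and clamping between the two limit angles.
; Tick also toggles LockStatus when the roll nears the opposite limit.
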(event `/Game/VirtualRealityBP/Blueprints/PickupActorInterface.Pickup`
  (params (AttachTo :type "SceneComponent Object Reference"))
  (set `self.Hand` AttachTo))

(event `/Game/VirtualRealityBP/Blueprints/PickupActorInterface.Drop`
  (`/Engine/EditorBlueprintResources/StandardMacros.IsValid` (`self.Hand`)
    (:`Is Valid`
      (set `self.Hand` null))))

(event `self.ReceiveTick`
  (params (DeltaSeconds :type "Float (single-precision)"))
  (bind _knob (`self.Knob`))
  (bind _knob_2 (`self.Knob`))
  (bind _relativerotation_roll (`KismetMathLibrary.BreakRotator` (`SceneComponent.RelativeRotation` (`self.Knob`))))
  (bind _relativerotation_roll_2 (`KismetMathLibrary.BreakRotator` (`SceneComponent.RelativeRotation` (`self.Knob`))))
  (bind _relativerotation_roll_3 (`KismetMathLibrary.BreakRotator` (`SceneComponent.RelativeRotation` _knob)))
  (bind _relativerotation_roll_4 (`KismetMathLibrary.BreakRotator` (`SceneComponent.RelativeRotation` _knob_2)))
  (bind (_returnvalue_roll _returnvalue_pitch) (`KismetMathLibrary.BreakRotator` (`SceneComponent.K2_GetComponentRotation` (`StaticMeshActor.StaticMeshComponent` (`self.Rod_Ref`)))))
  (`|ExecutionSequence`
    (:`then_0`
      ;[1 1 1] Update actor rotation (roll) according to hand position
      (bind _hand (`self.Hand`)
        (:`then`
          (if (`KismetMathLibrary.NearlyEqual_FloatFloat` _returnvalue_pitch 0.0 5.0)
            (bind (_returnvalue_roll_2 _returnvalue_pitch_2) (`KismetMathLibrary.BreakRotator` (`KismetMathLibrary.FindLookAtRotation` (`SceneComponent.K2_GetComponentLocation` (`self.Knob`)) (`SceneComponent.K2_GetComponentLocation` _hand))))
            (`SceneComponent.K2_SetRelativeRotation` _knob (`KismetMathLibrary.MakeRotator` (`KismetMathLibrary.FClamp` (- _relativerotation_roll_3 _returnvalue_pitch_2) (`self.unlockAngle`) (`self.lockAngle`))) false true)
            (else
              (bind (_returnvalue_roll_3 _returnvalue_pitch_3) (`KismetMathLibrary.BreakRotator` (`KismetMathLibrary.FindLookAtRotation` (`SceneComponent.K2_GetComponentLocation` _hand) (`SceneComponent.K2_GetComponentLocation` (`self.Knob`)))))
              (`SceneComponent.K2_SetRelativeRotation` _knob_2 (`KismetMathLibrary.MakeRotator` (`KismetMathLibrary.FClamp` (- _relativerotation_roll_4 _returnvalue_pitch_3) (`self.unlockAngle`) (`self.lockAngle`))) false true))))
        (:`else`)))
    (:`then_1`
      ;[1 1 1] Check knob status
      (switch `/Game/Aquilos/Blueprints/Enum_Lock_Status` (`self.lockStatus`)
        (:`NewEnumerator0`
          (if (`KismetMathLibrary.NearlyEqual_FloatFloat` _relativerotation_roll_2 (`self.unlockAngle`) 3.0)
            (set `self.lockStatus` "NewEnumerator1")))
        (:`NewEnumerator1`
          (if (`KismetMathLibrary.NearlyEqual_FloatFloat` _relativerotation_roll (`self.lockAngle`) 3.0)
            (set `self.lockStatus` "NewEnumerator0")))))))

(fn `UserConstructionScript`)