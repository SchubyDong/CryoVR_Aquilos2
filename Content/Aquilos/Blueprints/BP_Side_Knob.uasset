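; Hand-driven valve knob that must be rotated to unlock, slid between two spline points, then locked again.
; While held, its pitch follows the hand within the lock angles, and sliding follows the hand only near the unlock angle.
; Tick derives lock, slider and valve states, toggling the valve when locked at either end.
; Valve changes append non-repeating step IDs to the game instance, with rod knobs also checking rod attachment.
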(event `CheckLock`
  (bind (_relativerotation_roll _relativerotation_pitch) (`KismetMathLibrary.BreakRotator` (`SceneComponent.RelativeRotation` (`self.Knob`))))
  (bind (_relativerotation_roll_2 _relativerotation_pitch_2) (`KismetMathLibrary.BreakRotator` (`SceneComponent.RelativeRotation` (`self.Knob`))))
  ;[1 0.1882 0.1882] Check lock status
  (switch `/Game/Aquilos/Blueprints/Enum_Lock_Status` (`self.lockStatus`)
    (:`NewEnumerator0`
      (if (`KismetMathLibrary.NearlyEqual_FloatFloat` _relativerotation_pitch_2 (`self.unlockAngle`) 3.0)
        (set `self.lockStatus` "NewEnumerator1")))
    (:`NewEnumerator1`
      (if (`KismetMathLibrary.NearlyEqual_FloatFloat` _relativerotation_pitch (`self.lockAngle`) 3.0)
        (set `self.lockStatus` "NewEnumerator0")))))

(event `/Game/VirtualRealityBP/Blueprints/PickupActorInterface.Pickup`
  (params (AttachTo :type "SceneComponent Object Reference"))
  (set `self.Hand` AttachTo))

(event `/Game/VirtualRealityBP/Blueprints/PickupActorInterface.Drop`
  (`/Engine/EditorBlueprintResources/StandardMacros.IsValid` (`self.Hand`)
    (:`Is Valid`
      (set `self.Hand` null))))

(event `CheckSlider`
  ;[0.5137 1 0.4118] Check slider status
  (switch `/Game/Aquilos/Blueprints/Enum_Slider_Position` (`self.sliderPosition`)
    (:`NewEnumerator0`
      (if (== (`SceneComponent.K2_GetComponentLocation` (`self.Knob`)) (`SplineComponent.GetLocationAtSplinePoint` (`self.Spline`) 1 "World") :`ErrorTolerance` 2.0)
        (set `self.sliderPosition` "NewEnumerator1")))
    (:`NewEnumerator1`
      (if (== (`SceneComponent.K2_GetComponentLocation` (`self.Knob`)) (`SplineComponent.GetLocationAtSplinePoint` (`self.Spline`) 0 "World") :`ErrorTolerance` 2.0)
        (set `self.sliderPosition` "NewEnumerator0")))))

(event `self.ReceiveTick`
  (params (DeltaSeconds :type "Float (single-precision)"))
  (`|ExecutionSequence`
    (:`then_0`
      (`self.UpdateLockRotation`))
    (:`then_1`
      (`self.CheckLock`))
    (:`then_2`
      (`self.UpdateSliderPosition`))
    (:`then_3`
      (`self.CheckSlider`))
    (:`then_4`
      (`self.CheckValve`))))

(event `UpdateLockRotation`
  (bind _knob (`self.Knob`))
  (bind (_relativerotation_roll _relativerotation_pitch) (`KismetMathLibrary.BreakRotator` (`SceneComponent.RelativeRotation` _knob)))
  (if (`self.ifEnableRotate`)
    ;[1 0.1882 0.1882] Update knob rotation according to hand's rotation
    (bind _hand (`self.Hand`)
      (:`then`
        (bind (_returnvalue_roll _returnvalue_pitch) (`KismetMathLibrary.BreakRotator` (`KismetMathLibrary.FindLookAtRotation` (`SceneComponent.K2_GetComponentLocation` (`self.Knob`)) (`SceneComponent.K2_GetComponentLocation` _hand))))
        (`SceneComponent.K2_SetRelativeRotation` _knob (`KismetMathLibrary.MakeRotator` 0.0 (`KismetMathLibrary.FClamp` (+ _relativerotation_pitch _returnvalue_pitch) (`self.unlockAngle`) (`self.lockAngle`))) false true))
      (:`else`))))

(event `CheckValve`
  (bind _rod_ref (`self.Rod_Ref`))
  (bind _returnvalue (or (`|EnumEquality` (`/Game/Aquilos/Blueprints/BP_Rod.attachTo` _rod_ref) "NewEnumerator0") (`|EnumEquality` (`/Game/Aquilos/Blueprints/BP_Rod.attachTo` _rod_ref) "NewEnumerator1")))
  ;[0.391 1 0.8696] Check valve status
  (switch `/Game/Aquilos/Blueprints/Enum_Valve_Status` (`self.valveStatus`)
    (:`NewEnumerator1`
      (if (and (`|EnumEquality` (`self.lockStatus`) "NewEnumerator0") (`|EnumEquality` (`self.sliderPosition`) "NewEnumerator1"))
        (set `self.valveStatus` "NewEnumerator0")
        (if (`self.isRodKnob`)
          (if _returnvalue
            (`self.StepRecord` 3))
          (else
            (`self.StepRecord` 2)))))
    (:`NewEnumerator0`
      (if (and (`|EnumEquality` (`self.lockStatus`) "NewEnumerator0") (`|EnumEquality` (`self.sliderPosition`) "NewEnumerator0"))
        (set `self.valveStatus` "NewEnumerator1")
        (if (`self.isRodKnob`)
          (if _returnvalue
            (`self.StepRecord` 9))
          (else
            (`self.StepRecord` 10)))))))

(event `UpdateSliderPosition`
  (bind _spline (`self.Spline`))
  (bind (_relativerotation_roll _relativerotation_pitch) (`KismetMathLibrary.BreakRotator` (`SceneComponent.RelativeRotation` (`self.Knob`))))
  ;[1 1 1] Only enable sliding when unlock
  (bind _output_get (set `self.ifEnableSlide` (`KismetMathLibrary.NearlyEqual_FloatFloat` _relativerotation_pitch (`self.unlockAngle`) 3.0)))
  (if _output_get
    ;[0.5137 1 0.4118] Update knob location according to hand's location
    (bind _hand (`self.Hand`)
      (:`then`
        (`SceneComponent.K2_SetWorldLocation` (`self.Knob`) (`KismetMathLibrary.FindClosestPointOnSegment` (`SceneComponent.K2_GetComponentLocation` _hand) (`SplineComponent.GetLocationAtSplinePoint` _spline 0 "World") (`SplineComponent.GetLocationAtSplinePoint` _spline 1 "World")) false true))
      (:`else`))))

(fn `StepRecord`
  (params (Step :type Integer))
  (bind _asglobal_arrays (cast `/Game/CryoVR_GeneralContent/Blueprints/Global_Arrays` (`GameplayStatics.GetGameInstance`)))
  (bind _stepindexrecord (`/Game/CryoVR_GeneralContent/Blueprints/Global_Arrays.StepIndexRecord` _asglobal_arrays))
  (bind _returnvalue (`KismetArrayLibrary.Array_Length` _stepindexrecord))
  (if (> _returnvalue 0)
    (if (!= (`|GetArrayItem` _stepindexrecord (- _returnvalue 1)) Step)
      (`KismetArrayLibrary.Array_Add` _stepindexrecord Step))))

(fn `UserConstructionScript`)