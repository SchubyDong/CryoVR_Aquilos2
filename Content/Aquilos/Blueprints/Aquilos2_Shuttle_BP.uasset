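; Aquilos2 shuttle actor for a step-tracked workstation procedure, receiving a grid from tweezers.
; On overlapping the workstation's shuttle collision, it snaps to the platform's socket and flags itself attached.
; When tweezers overlap its grid collision and the workstation reports shuttle horizontal, grid on tweezer and screw loose, it swaps grid visibility from tweezers to shuttle.
; That swap also updates the workstation's grid status and records the step.
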(event `self.Shuttle_Collision.OnComponentBeginOverlap`
  (params (OverlappedComponent :type "PrimitiveComponent Object Reference") (OtherActor :type "Actor Object Reference") (OtherComp :type "PrimitiveComponent Object Reference") (OtherBodyIndex :type Integer) (bFromSweep :type Boolean) (SweepResult :type "HitResult Structure (by ref)"))
  (bind _asbp_workstation (cast `/Game/Aquilos/Blueprints/BP_Workstation` OtherActor))
  (if (== (`/Game/Aquilos/Blueprints/BP_Workstation.Shuttle_Collision` _asbp_workstation) OtherComp)
    (`self.K2_AttachToComponent` (`/Game/Aquilos/Blueprints/BP_Workstation.Shuttle_Platform` _asbp_workstation) "Shuttle_Socket" "SnapToTarget" "SnapToTarget" "KeepWorld")
    (set `self.Is_Shuttle_Attached` true)))

(event `self.Grid_Collision.OnComponentBeginOverlap`
  (params (OverlappedComponent :type "PrimitiveComponent Object Reference") (OtherActor :type "Actor Object Reference") (OtherComp :type "PrimitiveComponent Object Reference") (OtherBodyIndex :type Integer) (bFromSweep :type Boolean) (SweepResult :type "HitResult Structure (by ref)"))
  (bind _workstation (`self.workstation`))
  (bind _asbp_tweezers (cast `/Game/Aquilos/Blueprints/BP_Tweezers` OtherActor))
  (switch `/Game/Aquilos/Blueprints/Enum_Shuttle_Status` (`/Game/Aquilos/Blueprints/BP_Workstation.ShuttleStatus` _workstation)
    (:`NewEnumerator1`
      (switch `/Game/Aquilos/Blueprints/Enum_Grid_Status` (`/Game/Aquilos/Blueprints/BP_Workstation.GridStatus` _workstation)
        (:`NewEnumerator1`
          (switch `/Game/Aquilos/Blueprints/Enum_ShuttleScrew_Status` (`/Game/Aquilos/Blueprints/BP_Workstation.ShuttleScrewStatus` _workstation)
            (:`NewEnumerator1`
              (`SceneComponent.SetVisibility` (`/Game/Aquilos/Blueprints/BP_Tweezers.Grid` _asbp_tweezers) false false)
              (`SceneComponent.SetVisibility` (`self.Grid`) true false)
              (set `/Game/Aquilos/Blueprints/BP_Workstation.GridStatus` "NewEnumerator2" _workstation)
              (`self.StepRecord` 29))))))))

(fn `UserConstructionScript`
  (`parent.UserConstructionScript`))