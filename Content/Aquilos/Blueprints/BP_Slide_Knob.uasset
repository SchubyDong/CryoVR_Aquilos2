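; BP_Slide_Knob is a grabbable VR slider knob that moves between the two ends of a spline and records procedure steps.
; While held and RodBottomKnob is unlocked, Tick snaps the bottom knob to the hand's closest point on that segment.
; Reaching either end flips the slider state and logs step and time to Global_Arrays.
; A timeline animates an indication knob from IsInserting, and thumb presses while held toggle the top knob's lock position.
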(event `/Game/VirtualRealityBP/Blueprints/PickupActorInterface.Pickup`
  (params (AttachTo :type "SceneComponent Object Reference"))
  (set `self.Hand` AttachTo))

(event `/Game/VirtualRealityBP/Blueprints/PickupActorInterface.Drop`
  (`/Engine/EditorBlueprintResources/StandardMacros.IsValid` (`self.Hand`)
    (:`Is Valid`
      (set `self.Hand` null))))

(event `self.ReceiveTick`
  (params (DeltaSeconds :type "Float (single-precision)"))
  (bind _knob_top (`self.Knob_Top`))
  (bind _spline (`self.Spline`))
  (`|ExecutionSequence`
    (:`then_0`
      ;[1 1 1] Update slider location according to hand position
      (if (`|EnumEquality` (`/Game/Aquilos/Blueprints/BP_Bottom_Knob.lockStatus` (`self.RodBottomKnob`)) "NewEnumerator1")
        (bind _hand (`self.Hand`)
          (:`then`
            (`SceneComponent.K2_SetWorldLocation` (`self.Knob_Bottom`) (`KismetMathLibrary.FindClosestPointOnSegment` (`SceneComponent.K2_GetComponentLocation` _hand) (`SplineComponent.GetLocationAtSplinePoint` _spline 0 "World") (`SplineComponent.GetLocationAtSplinePoint` _spline 1 "World")) false true))
          (:`else`))))
    (:`then_1`
      ;[1 1 1] Check slider status
      (switch `/Game/Aquilos/Blueprints/Enum_Slider_Position` (`self.sliderPosition`)
        (:`NewEnumerator0`
          (if (== (`SceneComponent.K2_GetComponentLocation` (`self.Knob_Bottom`)) (`SplineComponent.GetLocationAtSplinePoint` (`self.Spline`) 1 "World") :`ErrorTolerance` 3.0)
            (set `self.sliderPosition` "NewEnumerator1")
            (`self.StepRecord` 5)))
        (:`NewEnumerator1`
          (if (== (`SceneComponent.K2_GetComponentLocation` (`self.Knob_Bottom`)) (`SplineComponent.GetLocationAtSplinePoint` (`self.Spline`) 0 "World") :`ErrorTolerance` 3.0)
            (set `self.sliderPosition` "NewEnumerator0")
            (`self.StepRecord` 6)))))
    (:`then_2`
      ;[1 1 1] Indication_Animation
      (if (`self.Is_Inserting`)
        (`self.Insert Rod Animation`)
        (else
          (`self.Pullout Rod Animation`))))
    (:`then_3`
      ;[1 1 1] Set Knob_Top Lock status
      (switch `/Game/Aquilos/Blueprints/Enum_Lock_Status` (`self.KnobTop_LockStatus`)
        (:`NewEnumerator0`
          (`SceneComponent.K2_SetRelativeLocation` _knob_top (0.0 0.0 1.261602) false false))
        (:`NewEnumerator1`
          (`SceneComponent.K2_SetRelativeLocation` _knob_top (0.0 0.0 1.831422) false false))))))

(event `Insert Rod Animation`
  ;[1 1 1] Indication_Animation
  (bind (_direction _alpha) (`Timeline|Timeline_0` :!label _label)
    (:`Update`
      (`SceneComponent.K2_SetWorldLocation` (`self.Indication_Knob`) (`KismetMathLibrary.VLerp` (`SplineComponent.GetLocationAtSplinePoint` (`self.Spline`) 0 "World") (`SplineComponent.GetLocationAtSplinePoint` (`self.Spline`) 1 "World") _alpha) false false))))

(event `Pullout Rod Animation`
  (goto _label :!via `Reverse`))

(event `InputAction|Thumb_Press_Left`
  (params (Key :type "Key Structure"))
  ;[1 1 1] Thumb_Press to Knob top
  (:`Pressed`
    (`self.Hand` :!label _label_2
      (:`then`
        (switch `/Game/Aquilos/Blueprints/Enum_Lock_Status` (`self.KnobTop_LockStatus`)
          (:`NewEnumerator0`
            (set `self.KnobTop_LockStatus` "NewEnumerator1")
            (`KismetSystemLibrary.PrintString` "Hello"))
          (:`NewEnumerator1`
            (set `self.KnobTop_LockStatus` "NewEnumerator0")
            (`KismetSystemLibrary.PrintString` "1111111111"))))
      (:`else`))))

(event `InputAction|Thumb_Press_Right`
  (params (Key :type "Key Structure"))
  ;[1 1 1] Thumb_Press to Knob top
  (:`Pressed`
    (goto _label_2)))

(fn `StepRecord`
  (params (Step :type Integer))
  (bind _asglobal_arrays (cast `/Game/CryoVR_GeneralContent/Blueprints/Global_Arrays` (`GameplayStatics.GetGameInstance`)))
  (bind _stepindexrecord (`/Game/CryoVR_GeneralContent/Blueprints/Global_Arrays.StepIndexRecord` _asglobal_arrays))
  (bind _returnvalue (`KismetArrayLibrary.Array_Length` _stepindexrecord))
  (if (> _returnvalue 0)
    (if (!= (`|GetArrayItem` _stepindexrecord (- _returnvalue 1)) Step)
      (`KismetArrayLibrary.Array_Add` _stepindexrecord Step)
      (`KismetArrayLibrary.Array_Add` (`/Game/CryoVR_GeneralContent/Blueprints/Global_Arrays.StepTimeRecord` _asglobal_arrays) (`/Game/CryoVR_GeneralContent/Blueprints/Global_Arrays.GlobalRecordTime` _asglobal_arrays)))))

(fn `UserConstructionScript`)