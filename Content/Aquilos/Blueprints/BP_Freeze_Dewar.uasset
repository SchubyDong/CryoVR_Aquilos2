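; Freeze dewar in the Aquilos workstation procedure, handling grid box pickup and placement (steps 14 and 15).
; When the dewar tweezer overlaps GridBox_Collision, the workstation's GridBoxStatus selects the transfer direction and flips between dewar and tweezer.
; The transfer is faked by swapping visibility of box and cap meshes on both actors.
; A DoOnce debounces overlaps, resetting one second after a transfer; any other status leaves it closed.
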(event `self.GridBox_Collision.OnComponentBeginOverlap`
  (params (OverlappedComponent :type "PrimitiveComponent Object Reference") (OtherActor :type "Actor Object Reference") (OtherComp :type "PrimitiveComponent Object Reference") (OtherBodyIndex :type Integer) (bFromSweep :type Boolean) (SweepResult :type "HitResult Structure (by ref)"))
  ;[1 1 1] Step 14 & 15 Pickup the gridbox & put gridbox into the pod
  (bind _asbp_freeze_dewar_tweezer (cast `/Game/Aquilos/Blueprints/BP_Freeze_Dewar_Tweezer` OtherActor))
  (`/Engine/EditorBlueprintResources/StandardMacros.DoOnce` false :!label _label
    (:`Completed`
      (switch `/Game/Aquilos/Blueprints/Enum_GridBox_Status` (`/Game/Aquilos/Blueprints/BP_Workstation.GridBoxStatus` (`self.Workstation_ref`))
        (:`NewEnumerator0`
          (`SceneComponent.SetVisibility` (`/Game/Aquilos/Blueprints/BP_Freeze_Dewar_Tweezer.GridBox` _asbp_freeze_dewar_tweezer) true false)
          (`SceneComponent.SetVisibility` (`/Game/Aquilos/Blueprints/BP_Freeze_Dewar_Tweezer.GridBoxCap` _asbp_freeze_dewar_tweezer) true false)
          (`SceneComponent.SetVisibility` (`self.GridBox`) false false)
          (`SceneComponent.SetVisibility` (`self.GridBoxCap`) false false)
          (set `/Game/Aquilos/Blueprints/BP_Workstation.GridBoxStatus` "NewEnumerator1" (`self.Workstation_ref`))
          (`KismetSystemLibrary.Delay` 1.0)
          (goto _label :!via `Reset`))
        (:`NewEnumerator1`
          (`SceneComponent.SetVisibility` (`/Game/Aquilos/Blueprints/BP_Freeze_Dewar_Tweezer.GridBox` _asbp_freeze_dewar_tweezer) false false)
          (`SceneComponent.SetVisibility` (`/Game/Aquilos/Blueprints/BP_Freeze_Dewar_Tweezer.GridBoxCap` _asbp_freeze_dewar_tweezer) false false)
          (`SceneComponent.SetVisibility` (`self.GridBox`) true false)
          (`SceneComponent.SetVisibility` (`self.GridBoxCap`) true false)
          (set `/Game/Aquilos/Blueprints/BP_Workstation.GridBoxStatus` "NewEnumerator0" (`self.Workstation_ref`))
          (`KismetSystemLibrary.Delay` 1.0)
          (goto _label :!via `Reset`))))))

(fn `UserConstructionScript`)