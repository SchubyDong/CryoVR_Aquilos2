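; Indication_Knob_BP is a knob actor that animates between pushed-in and pulled-out states based on its IsOpen flag.
; Tick checks the flag every frame and plays PulloutTimeline forward or in reverse.
; The timeline's two tracks slide the static mesh along world X and rotate its pitch a quarter turn.
; Endpoints are hard-coded world coordinates, so the motion is tied to one spot in the level.
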(event `self.ReceiveTick`
  (params (DeltaSeconds :type "Float (single-precision)"))
  (if (`self.Is_Open`)
    (`self.PulloutAnimation`)
    (else
      (`self.PushinAnimation`))))

(event `PulloutAnimation`
  (bind (_direction _pullout _rotate) (`Timeline|Pullout Timeline` :!label _label)
    (:`Update`
      (`SceneComponent.K2_SetWorldLocation` (`self.StaticMesh`) (`KismetMathLibrary.MakeVector` (`KismetMathLibrary.Lerp` 171.658386 164.255829 _pullout) -144.554092 150.577377) false false)
      (`SceneComponent.K2_SetRelativeRotation` (`self.StaticMesh`) (`KismetMathLibrary.MakeRotator` 0.0 (`KismetMathLibrary.Lerp` 90.0 0.0 _rotate) 90.0) false false))))

(event `PushinAnimation`
  (goto _label :!via `Reverse`))

(fn `UserConstructionScript`)