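; DewarCapActor is the cap for a dewar, reacting to VR hand contact.
; On BeginPlay it caches the game instance as Global_Arrays.
; When a motion controller overlaps its capsule, it calls UpdateHandAniFunc with gesture inputs and the TankCap_Socket snap socket.
; Unconnected nodes for attaching it to the dewar's CapSocket and recording step 4 never run.
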(event `self.ReceiveBeginPlay`
  (`parent.ReceiveBeginPlay`)
  (bind _asglobal_arrays (cast `/Game/CryoVR_GeneralContent/Blueprints/Global_Arrays` (`GameplayStatics.GetGameInstance`)))
  (set `self.GA` _asglobal_arrays))

(event `self.Capsule.OnComponentBeginOverlap`
  (params (OverlappedComponent :type "PrimitiveComponent Object Reference") (OtherActor :type "Actor Object Reference") (OtherComp :type "PrimitiveComponent Object Reference") (OtherBodyIndex :type Integer) (bFromSweep :type Boolean) (SweepResult :type "HitResult Structure (by ref)"))
  (`|ExecutionSequence`
    (:`then_0`
      (cast `/Game/VirtualRealityBP/Blueprints/BP_MotionController` OtherActor)
      (`self.UpdateHandAniFunc` null 0.33 0.8 "TankCap_Socket" "SnapToTarget"))))

(event `self.ReceiveTick`
  (params (DeltaSeconds :type "Float (single-precision)")))

(fn `UserConstructionScript`
  (`parent.UserConstructionScript`))